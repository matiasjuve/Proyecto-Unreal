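; Melee enemy that wanders until it senses or is shot by the player, then chases and damages them at close range.
; PawnSensing and bullet overlaps trigger AI MoveTo chases, and Tick keeps a wounded enemy pursuing.
; Delays on Tick act as timers for random roaming and distance-based attack checks.
; Each bullet removes fixed health, and death destroys the enemy and increments the player's kill count.
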(event `self.ReceiveActorBeginOverlap`
  (params (OtherActor :type "Actor Object Reference"))
  (bind _returnvalue (`GameplayStatics.GetPlayerCharacter` 0))
  ;[1 1 1] Getting shoot
  (cast `/Game/Blueprints/BP_Bullet_Base` OtherActor)
  (set `self.CanSeePlayer` true)
  (set `self.Current Health` (- (`self.Current Health`) 0.25))
  (if (<= (`self.Current Health`) 0.0)
    (bind _asbp_my_character (cast `/Game/Blueprints/BP_MyCharacter` _returnvalue))
    (`self.K2_DestroyActor`)
    (bind _result (`/Engine/EditorBlueprintResources/StandardMacros.IncrementInt` (`/Game/Blueprints/BP_MyCharacter.KillCount` _asbp_my_character))
      (:`  `
        (`KismetSystemLibrary.PrintString` (`KismetStringLibrary.Conv_IntToString` _result))))
    (else
      (bind _asbp_my_character_2 (cast `/Game/Blueprints/BP_MyCharacter` _returnvalue))
      (`|AIMoveTo` self (0.0 0.0 0.0) _asbp_my_character_2
        (:`OnSuccess`
          _)
        (:`OnFail`
          _))
      (set `self.CanSeePlayer` false))))

(event `self.ReceiveTick`
  (params (DeltaSeconds :type "Float (single-precision)"))
  (bind _current_health (`self.Current Health`))
  (`|ExecutionSequence`
    (:`then_0`
      (`KismetSystemLibrary.Delay` 2.0)
      (if (not (`self.CanSeePlayer`))
        (`|AIMoveTo` self (`NavigationSystemV1.K2_GetRandomReachablePointInRadius` (`self.K2_GetActorLocation`) 250.0 null null) null)))
    (:`then_1`
      (bind _asbp_my_character (cast `/Game/Blueprints/BP_MyCharacter` (`GameplayStatics.GetPlayerCharacter` 0)))
      (`KismetSystemLibrary.Delay` 0.5)
      (if (<= (`self.GetDistanceTo` _asbp_my_character) 150.0)
        (set `self.Hit` true)
        (`/Game/Blueprints/BP_MyCharacter.TakeDamage` _asbp_my_character)
        (else
          (set `self.Hit` false))))
    (:`then_2`
      (if (!= _current_health 1.0)
        (if (not (<= _current_health 0.0))
          (bind _asbp_my_character_2 (cast `/Game/Blueprints/BP_MyCharacter` (`GameplayStatics.GetPlayerCharacter` 0)))
          (`|AIMoveTo` self (0.0 0.0 0.0) _asbp_my_character_2))))))

(event `self.PawnSensing.OnSeePawn`
  (params (Pawn :type "Pawn Object Reference"))
  (set `self.CanSeePlayer` true)
  (bind _asbp_my_character (cast `/Game/Blueprints/BP_MyCharacter` (`GameplayStatics.GetPlayerCharacter` 0)))
  (`|AIMoveTo` self (0.0 0.0 0.0) _asbp_my_character
    (:`then`
      (`KismetSystemLibrary.Delay` 2.0))))

(fn `UserConstructionScript`)