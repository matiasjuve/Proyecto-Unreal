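; Player character for a shooter, with a weapon, armor and health, HUD and crosshair, and physics-object grabbing.
; Input drives looped firing, reload, sprint and aim-down-sights camera switching, while a line trace feeds a PhysicsHandle for grab and drop.
; Bullet overlaps and damage functions drain armor and health.
; Tick regenerates armor after a delay, scales crosshair spread with speed, switches the objective to the boss by kill count and opens Defeat on death.
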(event `self.ReceiveActorBeginOverlap`
  (params (OtherActor :type "Actor Object Reference"))
  ;[1 1 1] Receive bullet damage
  (cast `/Game/Blueprints/BP_Enemy_Bullet` OtherActor)
  (if (<= (`self.Armor`) 0.0)
    (set `self.Health` (- (`self.Health`) 0.25))
    (else
      (set `self.Armor` (- (`self.Armor`) 0.25))
      (set `self.Safe` false))))

(event `self.ReceiveBeginPlay`
  (bind _returnvalue (`|CreateWidget` "/Game/Blueprints/BP_UI.BP_UI_C"))
  (`UserWidget.AddToViewport` _returnvalue 0)
  (bind _returnvalue_2 (`|CreateWidget` "/Game/Crosshair/DynamicCrossHair.WBCrosshair_C"))
  (bind _output_get (set `self.CrosshairReference` _returnvalue_2))
  (`UserWidget.AddToViewport` _returnvalue_2 0)
  (`UserWidget.AddToViewport` _output_get 0)
  (bind _returnvalue_3 (`|SpawnActorFromClass` "/Game/Blueprints/Weapon/Ak-47/Weapon_Base.Weapon_Base_C" (`KismetMathLibrary.MakeTransform` (0.0 0.0 0.0)) "Undefined" "OverrideRootScale" null null))
  (bind _output_get_2 (set `self.Equiped_Weapon` _returnvalue_3))
  (`self.K2_AttachToComponent` _output_get_2 (`self.Mesh`) "Weapon_Attach" "KeepRelative" "KeepRelative" "KeepRelative" true))

(event `self.ReceiveTick`
  (params (DeltaSeconds :type "Float (single-precision)"))
  (`|ExecutionSequence`
    (:`then_0`
      (`KismetSystemLibrary.Delay` 3.0 :!label _label)
      (bind _output_get (set `self.Safe` true))
      (if (and _output_get (< (`self.Armor`) 1.0))
        (set `self.Armor` (+ (`self.Armor`) 0.05))
        (goto _label)))
    (:`then_1`
      (set `/Game/Crosshair/DynamicCrossHair.crosshair_spread` (`KismetMathLibrary.MapRangeClamped` (`KismetMathLibrary.VSize` (`self.GetVelocity`)) 0.0 450.0 5.0 80.0) (`self.CrosshairReference`)))
    (:`then_2`
      ;[1 1 1] Enemy count
      (if (>= (`self.KillCount`) 13)
        (set `self.ObjetiveText` "Fight the boss")))
    (:`then_3`
      ;[1 1 1] Raycast
      (`PhysicsHandleComponent.SetTargetLocation` (`self.PhysicsHandle`) (`SceneComponent.K2_GetComponentLocation` (`self.HeldObject`))))
    (:`then_4`
      (if (<= (`self.Health`) 0.0)
        (`GameplayStatics.OpenLevel` "Defeat")))))

(event `InputAction|Primary_Fire`
  (params (Key :type "Key Structure"))
  (bind _equiped_weapon (`self.Equiped_Weapon`))
  ;[1 1 1] Shoot
  (:`Pressed`
    (if (> (`/Game/Blueprints/Weapon/Ak-47/Weapon_Base.Ammo` (`self.Equiped_Weapon`)) 0) :!label _label_2
      (set `self.IsFiring` true)
      (`/Game/Blueprints/Weapon/Ak-47/Weapon_Base.Fire` _equiped_weapon)
      (`KismetSystemLibrary.Delay` (`/Game/Blueprints/Weapon/Ak-47/Weapon_Base.FireRate` _equiped_weapon))
      (if (`self.IsFiring`)
        (goto _label_2))))
  (:`Released`
    (set `self.IsFiring` false)))

(event `InputAction|Reload`
  (params (Key :type "Key Structure"))
  ;[1 1 1] Reload
  (:`Pressed`
    (`/Game/Blueprints/Weapon/Ak-47/Weapon_Base.Reload` (`self.Equiped_Weapon`))))

(event `InputAction|ADS`
  (params (Key :type "Key Structure"))
  (:`Pressed`
    (if (`self.SprintTrue`)
      (set `self.SprintTrue` false)
      ;[1 1 1] ADS
      (set `CharacterMovementComponent.MaxWalkSpeed` 600.0 (`self.CharacterMovement`)))
    (`ActorComponent.Deactivate` (`self.CameraFollows`))
    (`ActorComponent.Activate` (`self.ADSCamera`) false)
    (set `CharacterMovementComponent.MaxWalkSpeed` 0.0 (stale _charactermovement))
    (set `self.isAimingSight` true))
  (:`Released`
    (bind _charactermovement (`self.StopADS`))))

(event `Key|E`
  (params (Key :type "Key Structure"))
  ;[1 1 1] Raycast
  (:`Pressed`
    (if (`self.IsHoldingObject`)
      (`self.DropObject`)
      (else
        (`self.GrabObject`)))))

(event `GrabObject`
  (bind _camerafollows (`self.CameraFollows`))
  (bind _returnvalue (`SceneComponent.K2_GetComponentLocation` _camerafollows))
  ;[1 1 1] Raycast
  (bind (_outhit _returnvalue_2) (`KismetSystemLibrary.LineTraceSingle` :`Start` _returnvalue :`End` (+ (* (`SceneComponent.GetForwardVector` _camerafollows) 100.0) _returnvalue) :`TraceChannel` "TraceTypeQuery1" :`DrawDebugType` "ForDuration"))
  (if _returnvalue_2
    (bind (_bblockinghit _binitialoverlap _time _distance _location _impactpoint _normal _impactnormal _physmat _hitactor _hitcomponent) (`GameplayStatics.BreakHitResult` _outhit))
    (if (`SceneComponent.IsSimulatingPhysics` _hitcomponent "None")
      (`PhysicsHandleComponent.GrabComponentAtLocation` (`self.PhysicsHandle`) _hitcomponent "None" (`SceneComponent.K2_GetComponentLocation` _hitcomponent))
      (set `self.IsHoldingObject` true))))

(event `InputAction|Sprint`
  (params (Key :type "Key Structure"))
  (:`Pressed`
    (if (`self.isAimingSight`)
      (`self.StopADS`))
    (set `self.SprintTrue` true)
    (set `CharacterMovementComponent.MaxWalkSpeed` 1000.0 (`self.CharacterMovement`)))
  (:`Released`
    (set `self.SprintTrue` false)
    (set `CharacterMovementComponent.MaxWalkSpeed` 600.0 (`self.CharacterMovement`))))

(event `DropObject`
  ;[1 1 1] Raycast
  (`PhysicsHandleComponent.ReleaseComponent` (`self.PhysicsHandle`))
  (set `self.IsHoldingObject` false))

(fn `CheckKillCount`
  (if (>= (`self.KillCount`) 2)
    (`KismetSystemLibrary.PrintString` "Ganaste")))

(fn `StopADS`
  (returns (CharacterMovement :type "CharacterMovementComponent Object Reference"))
  (bind _charactermovement (`self.CharacterMovement`))
  (`ActorComponent.Deactivate` (`self.ADSCamera`))
  (`ActorComponent.Activate` (`self.CameraFollows`) false)
  (set `CharacterMovementComponent.MaxWalkSpeed` 600.0 _charactermovement)
  (set `self.isAimingSight` false)
  (return _charactermovement))

(fn `TakeBossDamage`
  (bind _output_get (set `self.Armor` (- (`self.Armor`) 0.15)))
  (if (< _output_get 0.0)
    (set `self.Health` (- (`self.Health`) 0.15))))

(fn `TakeDamage`
  (bind _output_get (set `self.Armor` (- (`self.Armor`) 0.05)))
  (if (< _output_get 0.0)
    (set `self.Health` (- (`self.Health`) 0.15))))

(fn `UserConstructionScript`)