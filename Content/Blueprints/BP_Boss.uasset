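; Boss enemy that wanders randomly, chases the player and opens the "Win" level when its health runs out.
; Bullet overlaps reduce health and trigger a chase, whose completion or failure clears CanSeePlayer to resume wandering.
; Pawn sensing also starts a chase and, after a delay, spawns a melee minion at a random nearby reachable point.
; Tick uses Delays to throttle wandering and proximity attacks that damage the player.
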(event `self.ReceiveActorBeginOverlap`
  (params (OtherActor :type "Actor Object Reference"))
  (cast `/Game/Blueprints/BP_Bullet_Base` OtherActor)
  (set `self.CanSeePlayer` true)
  (set `self.CurrentHealt` (- (`self.CurrentHealt`) 0.25))
  (if (<= (`self.CurrentHealt`) 0.0)
    ;[1 1 1] Cambio de escena
    (`GameplayStatics.OpenLevel` "Win")
    (else
      (bind _asbp_my_character (cast `/Game/Blueprints/BP_MyCharacter` (`GameplayStatics.GetPlayerCharacter` 0)))
      (`|AIMoveTo` self (0.0 0.0 0.0) _asbp_my_character
        (:`OnSuccess`
          _)
        (:`OnFail`
          _))
      (set `self.CanSeePlayer` false))))

(event `self.ReceiveTick`
  (params (DeltaSeconds :type "Float (single-precision)"))
  (`|ExecutionSequence`
    (:`then_0`
      (`KismetSystemLibrary.Delay` 2.0)
      (if (not (`self.CanSeePlayer`))
        (`|AIMoveTo` self (`NavigationSystemV1.K2_GetRandomReachablePointInRadius` (`self.K2_GetActorLocation`) 250.0 null null) null)))
    (:`then_1`
      (bind _asbp_my_character (cast `/Game/Blueprints/BP_MyCharacter` (`GameplayStatics.GetPlayerCharacter` 0)))
      (`KismetSystemLibrary.Delay` 0.5)
      (if (<= (`self.GetDistanceTo` _asbp_my_character) 150.0)
        (set `self.Hit` true)
        (`/Game/Blueprints/BP_MyCharacter.TakeBossDamage` _asbp_my_character)
        (else
          (set `self.Hit` false))))))

(event `self.PawnSensing.OnSeePawn`
  (params (Pawn :type "Pawn Object Reference"))
  (`|ExecutionSequence`
    (:`then_0`
      (set `self.CanSeePlayer` true)
      (bind _asbp_my_character (cast `/Game/Blueprints/BP_MyCharacter` (`GameplayStatics.GetPlayerCharacter` 0)))
      (`|AIMoveTo` self (0.0 0.0 0.0) _asbp_my_character))
    (:`then_1`
      (`KismetSystemLibrary.Delay` 4.0)
      (`|SpawnActorFromClass` "/Game/Blueprints/BP_Enemy_Melee.BP_Enemy_Melee_C" (`KismetMathLibrary.Conv_VectorToTransform` (`NavigationSystemV1.K2_GetRandomReachablePointInRadius` (`self.K2_GetActorLocation`) 500.0 null null)) "Undefined" "OverrideRootScale" null null))))

(fn `UserConstructionScript`)