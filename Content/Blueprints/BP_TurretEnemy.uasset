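; Turret enemy that turns toward the player and fires bullets when it senses a pawn.
; BeginPlay spawns a Weapon_Base and calls an attach to the Mesh's "Weapon" socket, while Tick rotates the whole actor toward BP_MyCharacter.
; PawnSensing's OnSeePawn spawns a BP_Enemy_Bullet at the actor's transform; the trailing Delay gates nothing, so sensing events set the fire rate.
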(event `self.ReceiveBeginPlay`
  (`|SpawnActorFromClass` "/Game/Blueprints/Weapon/Ak-47/Weapon_Base.Weapon_Base_C" (`KismetMathLibrary.MakeTransform` (0.0 0.0 0.0) (struct) (0.0 0.0 0.0)) "Undefined" "OverrideRootScale" null null)
  (`self.K2_AttachToComponent` (`self.Mesh`) "Weapon" "KeepRelative" "KeepRelative" "KeepRelative"))

(event `self.ReceiveTick`
  (params (DeltaSeconds :type "Float (single-precision)"))
  ;[1 1 1] Pa mirar al player
  (bind _asbp_my_character (cast `/Game/Blueprints/BP_MyCharacter` (`GameplayStatics.GetPlayerCharacter` 0)))
  (`self.K2_SetActorRotation` (`KismetMathLibrary.FindLookAtRotation` (`self.K2_GetActorLocation`) (`self.K2_GetActorLocation` _asbp_my_character))))

(event `self.PawnSensing.OnSeePawn`
  (params (Pawn :type "Pawn Object Reference"))
  (`|SpawnActorFromClass` "/Game/Blueprints/BP_Enemy_Bullet.BP_Enemy_Bullet_C" (`self.GetTransform`) "Undefined" "OverrideRootScale" null null)
  (`KismetSystemLibrary.Delay` 0.75))

(fn `UserConstructionScript`)